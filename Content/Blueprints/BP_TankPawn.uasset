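; BP_TankPawn is a tank pawn Blueprint that connects its health to the player-facing UI.
; On BeginPlay it casts player pawn 0 to BP_TankPawn and, if valid, pushes current and max health from the health component to the tank health widget.
; When the health component fires OnDie, it creates a WBP_GameOver widget and adds it to the viewport.
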(event OnDie(Health_component)
  (bind _returnvalue (UserInterface|CreateWidget "/Game/Blueprints/WIdget/WBP_GameOver.WBP_GameOver_C"))
  (bind _output_get (Variables|Default|SetGame%20Over _returnvalue))
  (UserInterface|Viewport|AddtoViewport _output_get 0))

(event EventBeginPlay
  (bind _health_component (Variables|Default|GetHealth_component))
  (bind _asbp_tank_pawn (Utilities|Casting|CastToBP_TankPawn (Game|Player|GetPlayerPawn 0)))
  (bind _output_get (Variables|Default|SetPawn _asbp_tank_pawn))
  (Utilities|IsValid _output_get
    (:Is%20Valid
      (Default|UpdateHealth (Variables|Default|GetWTank%20Health) (Variables|/Script/Tankogeddon.HealthComponent|GetCurrentHealth _health_component) (Variables|/Script/Tankogeddon.HealthComponent|GetMaxHealth _health_component)))))

(fn ConstructionScript)